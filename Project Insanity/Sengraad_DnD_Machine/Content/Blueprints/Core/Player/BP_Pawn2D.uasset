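; BP_Pawn2D is a player pawn for a 2D view with an orthographic camera, supporting zoom and drag panning.
; On BeginPlay it adds the 2D Enhanced Input mapping context and seeds the desired zoom from the spring arm length.
; Zoom input adjusts a clamped target, while dragging converts mouse offset into a target location and shows a grab cursor.
; Tick smoothly interpolates ortho width and actor location toward those targets.
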(event Input|EnhancedActionEvents|EnhancedInputActionIA_Zoom
  (params (ActionValue :type Float%20%28double-precision%29) (ElapsedSeconds :type Float%20%28double-precision%29) (TriggeredSeconds :type Float%20%28double-precision%29) (InputAction :type Input%20Action%20Object%20Reference :default "/Game/Blueprints/Core/Player/Inputs/IA_Zoom.IA_Zoom"))
  (Variables|Default|SetZoom_Desired (Math|Float|Clamp(Float) (+ (* ActionValue 2e+02) (Variables|Default|GetZoom_Desired)) 5e+02 1e+04)))

(event Input|EnhancedActionEvents|EnhancedInputActionIA_DragMove
  (params (ActionValue :type Boolean) (ElapsedSeconds :type Float%20%28double-precision%29) (TriggeredSeconds :type Float%20%28double-precision%29) (InputAction :type Input%20Action%20Object%20Reference :default "/Game/Blueprints/Core/Player/Inputs/IA_DragMove.IA_DragMove"))
  (bind _returnvalue (Game|GetPlayerController 0))
  (:Triggered
    (bind _returnvalue_2 (Class|WidgetLayoutLibrary|GetMousePositiononViewport))
    (Variables|Default|SetCurrentMouseLocation _returnvalue_2)
    (Variables|Default|SetLocation_Desired (+ (Math|Vector|MakeVector (.y (- (Variables|Default|GetCurrentMouseLocation) (Variables|Default|GetStartMouseLocation))) (* (.x (- (Variables|Default|GetCurrentMouseLocation) (Variables|Default|GetStartMouseLocation))) -1.0) 0.0) (Transformation|GetActorLocation))))
  (:Started
    (Variables|/Script/Engine.PlayerController|SetCurrentMouseCursor _returnvalue "GrabHandClosed")
    (bind _returnvalue_3 (Class|WidgetLayoutLibrary|GetMousePositiononViewport))
    (Variables|Default|SetStartMouseLocation _returnvalue_3))
  (:Canceled
    (Variables|/Script/Engine.PlayerController|SetCurrentMouseCursor _returnvalue "Default" :!label _label))
  (:Completed
    (goto _label)))

(event EventBeginPlay
  (bind _asplayer_controller (Utilities|Casting|CastToPlayerController (Pawn|GetController)))
  (Utilities|IsValid (PlayerController|LocalPlayerSubsystems|GetEnhancedInputLocalPlayerSubsystem _asplayer_controller)
    (:Is%20Valid
      (Input|AddMappingContext (PlayerController|LocalPlayerSubsystems|GetEnhancedInputLocalPlayerSubsystem _asplayer_controller) "/Game/Blueprints/Core/Player/Inputs/IMC_2D.IMC_2D" 0 "(bIgnoreAllPressedKeysUntilRelease=True,bForceImmediately=False,bNotifyUserSettings=False)")
      (Variables|Default|SetStartMouseLocation "")
      (Variables|Default|SetZoom_Desired (Variables|/Script/Engine.SpringArmComponent|GetTargetArmLength (Variables|Default|GetSpringArm))))))

(event EventTick
  (params (DeltaSeconds :type Float%20%28single-precision%29))
  (bind _camera (Variables|Default|GetCamera))
  (Class|CameraComponent|SetOrthoWidth _camera (Math|Interpolation|FInterpTo (Variables|/Script/Engine.CameraComponent|GetOrthoWidth _camera) (Variables|Default|GetZoom_Desired) DeltaSeconds 1e+01))
  (Transformation|SetActorLocation (Math|Interpolation|VInterpTo (Transformation|GetActorLocation) (Variables|Default|GetLocation_Desired) DeltaSeconds 1e+01) false false))

(fn ConstructionScript)