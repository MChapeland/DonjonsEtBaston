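; BP_PC is a player controller that creates the player's HUD and relays session chat messages.
; On BeginPlay it enables the mouse cursor and adds the W_PCUI widget to the viewport.
; SetPlayerInformation stores name and image, then after a short delay broadcasts a welcome message.
; TransferMessage loops through BP_GM's ConnectedPlayers, and each one passes the message data to its HUD chat log.
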(event Custom|SetPlayerInformation
  (params (NewName :type String) (NewImage :type Texture%20Object%20Reference))
  ;[1 1 1] Initialization
  (bind _output_get (Variables|Default|SetPlayerName NewName))
  (Variables|Default|SetPlayerImage NewImage)
  (Utilities|FlowControl|Delay 0.5)
  (CallFunction|WelcomePlayer _output_get))

(event Custom|InitializeHUD
  ;[1 1 1] UI
  (bind _returnvalue (UserInterface|CreateWidget "/Game/Blueprints/UI/W_PCUI.W_PCUI_C" self))
  (bind _output_get (Variables|Default|SetHUDRef _returnvalue))
  (UserInterface|Viewport|AddtoViewport _output_get 0))

(event Custom|Transfer%20Message
  (params (Text :type String) (Type :type E_MessageTypes%20Enum :default "NewEnumerator1"))
  ;[1 1 1] UI
  ;;[1 1 1] Chat Functionality
  (bind _asbp_gm (Utilities|Casting|CastToBP_GM (Game|GetGameMode)))
  (for _array_element (Variables|/Game/Blueprints/Core/Player/BP_GM.BP_GM_C|GetConnectedPlayers _asbp_gm)
    (CallFunction|SendMessagetoChatLog _array_element (Variables|Default|GetPlayerName) (Variables|Default|GetPlayerImage) Text Type)))

(event Custom|Send%20Message%20to%20Chat%20Log
  (params (PlayerName :type String) (PlayerImage :type Texture%20Object%20Reference) (Message :type String) (Type :type E_MessageTypes%20Enum :default "NewEnumerator1"))
  ;[1 1 1] UI
  ;;[1 1 1] Chat Functionality
  (Default|ParseMessage (Variables|/Game/Blueprints/UI/W_PCUI.W_PCUI_C|GetW_ChatLog (Variables|Default|GetHUDRef)) (Utilities|Struct|MakeS_MessageData PlayerName PlayerImage Message Type)))

(event EventBeginPlay
  ;[1 1 1] Initialization
  (Variables|Default|SetbShowMouseCursor true)
  (Variables|Default|SetbEnableMouseOverEvents true)
  (CallFunction|InitializeHUD))

(fn ConstructionScript)

(fn WelcomePlayer
  (params (Player%20Name :type String))
  (CallFunction|TransferMessage (Utilities|String|ToString(Text) (Utilities|Text|FormatText "Welcome to the session {Player}!" Player%20Name)) "NewEnumerator8"))