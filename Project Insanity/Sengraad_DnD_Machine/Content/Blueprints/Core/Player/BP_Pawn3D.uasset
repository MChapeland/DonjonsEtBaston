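; BP_Pawn3D is a player camera pawn with a spring arm, offering panning, zooming, stepped yaw rotation and a top-down view toggle.
; BeginPlay adds the IMC_3D mapping context and seeds desired values, which Enhanced Input actions change and Tick smoothly interpolates toward.
; Pan speed scales with arm length, and outside top view the pitch steepens as the camera zooms out.
; Desired FOV is interpolated but never changed after initialization.
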(event Input|EnhancedActionEvents|EnhancedInputActionIA_Zoom
  (params (ActionValue :type Float%20%28double-precision%29) (ElapsedSeconds :type Float%20%28double-precision%29) (TriggeredSeconds :type Float%20%28double-precision%29) (InputAction :type Input%20Action%20Object%20Reference :default "/Game/Blueprints/Core/Player/Inputs/IA_Zoom.IA_Zoom"))
  (bind _output_get (Variables|Default|SetZoom_Desired (Math|Float|Clamp(Float) (+ (* ActionValue 2e+02) (Variables|Default|GetZoom_Desired)) 1e+03 4e+03)))
  (if (not (Variables|Default|GetTopView))
    (Variables|Default|SetViewAngle_Desired (+ (* (/ (- _output_get 1e+03) 3e+03) -3e+01) -3e+01))))

(event Input|EnhancedActionEvents|EnhancedInputActionIA_SwitchView
  (params (ActionValue :type Boolean) (ElapsedSeconds :type Float%20%28double-precision%29) (TriggeredSeconds :type Float%20%28double-precision%29) (InputAction :type Input%20Action%20Object%20Reference :default "/Game/Blueprints/Core/Player/Inputs/IA_SwitchView.IA_SwitchView"))
  (:Started
    (if (Variables|Default|GetTopView)
      (Variables|Default|SetTopView false)
      (Variables|Default|SetViewAngle_Desired -6e+01)
      (Variables|Default|SetViewAngle_Desired (+ (* (/ (- (Variables|Default|GetZoom_Desired) 1e+03) 3e+03) -3e+01) -3e+01))
      (else
        (Variables|Default|SetTopView true)
        (Variables|Default|SetViewAngle_Desired -9e+01)))))

(event Input|EnhancedActionEvents|EnhancedInputActionIA_MoveHorizontal
  (params (ActionValue :type Float%20%28double-precision%29) (ElapsedSeconds :type Float%20%28double-precision%29) (TriggeredSeconds :type Float%20%28double-precision%29) (InputAction :type Input%20Action%20Object%20Reference :default "/Game/Blueprints/Core/Player/Inputs/IA_MoveHorizontal.IA_MoveHorizontal"))
  (Variables|Default|SetLocation_Desired (+ (Variables|Default|GetLocation_Desired) (* (Transformation|GetActorForwardVector) (* ActionValue (/ (Variables|/Script/Engine.SpringArmComponent|GetTargetArmLength (Variables|Default|GetSpringArm)) 5e+01))))))

(event Input|EnhancedActionEvents|EnhancedInputActionIA_MoveVertical
  (params (ActionValue :type Float%20%28double-precision%29) (ElapsedSeconds :type Float%20%28double-precision%29) (TriggeredSeconds :type Float%20%28double-precision%29) (InputAction :type Input%20Action%20Object%20Reference :default "/Game/Blueprints/Core/Player/Inputs/IA_MoveVertical.IA_MoveVertical"))
  (Variables|Default|SetLocation_Desired (+ (Variables|Default|GetLocation_Desired) (* (Transformation|GetActorRightVector) (* (/ (Variables|/Script/Engine.SpringArmComponent|GetTargetArmLength (Variables|Default|GetSpringArm)) 5e+01) ActionValue)))))

(event Input|EnhancedActionEvents|EnhancedInputActionIA_Rotate
  (params (ActionValue :type Float%20%28double-precision%29) (ElapsedSeconds :type Float%20%28double-precision%29) (TriggeredSeconds :type Float%20%28double-precision%29) (InputAction :type Input%20Action%20Object%20Reference :default "/Game/Blueprints/Core/Player/Inputs/IA_Rotate.IA_Rotate"))
  (:Started
    (Variables|Default|SetRotation_Desired (Math|Rotator|CombineRotators (Variables|Default|GetRotation_Desired) (Math|Rotator|MakeRotator 0.0 0.0 (* ActionValue -45.0))))))

(event EventBeginPlay
  (bind _asplayer_controller (Utilities|Casting|CastToPlayerController (Pawn|GetController)))
  (Utilities|IsValid (PlayerController|LocalPlayerSubsystems|GetEnhancedInputLocalPlayerSubsystem _asplayer_controller)
    (:Is%20Valid
      (Input|AddMappingContext (PlayerController|LocalPlayerSubsystems|GetEnhancedInputLocalPlayerSubsystem _asplayer_controller) "/Game/Blueprints/Core/Player/Inputs/IMC_3D.IMC_3D" 0 "(bIgnoreAllPressedKeysUntilRelease=True,bForceImmediately=False,bNotifyUserSettings=False)")
      (Variables|Default|SetLocation_Desired (Transformation|GetActorLocation))
      (Variables|Default|SetZoom_Desired (Variables|/Script/Engine.SpringArmComponent|GetTargetArmLength (Variables|Default|GetSpringArm)))
      (Variables|Default|SetRotation_Desired (Transformation|GetActorRotation))
      (Variables|Default|SetFOV_Desired (Variables|/Script/Engine.CameraComponent|GetFieldOfView (Variables|Default|GetCamera)))
      (Variables|Default|SetViewAngle_Desired (.Pitch (Math|Rotator|BreakRotator (Variables|/Script/Engine.SceneComponent|GetRelativeRotation (Variables|Default|GetSpringArm))))))))

(event EventTick
  (params (DeltaSeconds :type Float%20%28single-precision%29))
  (bind _springarm (Variables|Default|GetSpringArm))
  (bind _camera (Variables|Default|GetCamera))
  (bind _springarm_2 (Variables|Default|GetSpringArm))
  (Variables|/Script/Engine.SpringArmComponent|SetTargetArmLength _springarm (Math|Interpolation|FInterpTo (Variables|/Script/Engine.SpringArmComponent|GetTargetArmLength _springarm) (Variables|Default|GetZoom_Desired) DeltaSeconds 1e+01))
  (Transformation|SetActorLocation (Math|Interpolation|VInterpTo (Transformation|GetActorLocation) (Variables|Default|GetLocation_Desired) DeltaSeconds 1e+01) false false)
  (Transformation|SetActorRotation (Math|Interpolation|RInterpTo (Transformation|GetActorRotation) (Variables|Default|GetRotation_Desired) DeltaSeconds 1e+01))
  (Camera|SetFieldOfView _camera (Math|Interpolation|FInterpTo (Variables|/Script/Engine.CameraComponent|GetFieldOfView _camera) (Variables|Default|GetFOV_Desired) DeltaSeconds 1e+01))
  (Transformation|SetRelativeRotation _springarm_2 (Math|Interpolation|RInterpTo (Variables|/Script/Engine.SceneComponent|GetRelativeRotation _springarm_2) (Math|Rotator|MakeRotator 0.0 (Variables|Default|GetViewAngle_Desired) 0.0) DeltaSeconds 1e+01) false false))

(fn ConstructionScript)