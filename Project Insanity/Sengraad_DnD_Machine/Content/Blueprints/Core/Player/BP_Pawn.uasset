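; Player camera pawn that pans, zooms and rotates through Enhanced Input, using a mapping context added on BeginPlay.
; Input events only update desired location, yaw and spring arm length, with clamped zoom and stepped rotation on press.
; Tick eases the actor transform and arm length toward those targets with interpolation.
; Pan speed scales with current arm length, so movement is faster when zoomed out.
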(event Input|EnhancedActionEvents|EnhancedInputActionIA_Zoom
  (params (ActionValue :type Float%20%28double-precision%29) (ElapsedSeconds :type Float%20%28double-precision%29) (TriggeredSeconds :type Float%20%28double-precision%29) (InputAction :type Input%20Action%20Object%20Reference :default "/Game/Blueprints/Core/Player/Inputs/IA_Zoom.IA_Zoom"))
  (Variables|Default|SetZoom_Desired (Math|Float|Clamp(Float) (+ (* ActionValue 2e+02) (Variables|Default|GetZoom_Desired)) 1e+03 4e+03)))

(event Input|EnhancedActionEvents|EnhancedInputActionIA_MoveHorizontal
  (params (ActionValue :type Float%20%28double-precision%29) (ElapsedSeconds :type Float%20%28double-precision%29) (TriggeredSeconds :type Float%20%28double-precision%29) (InputAction :type Input%20Action%20Object%20Reference :default "/Game/Blueprints/Core/Player/Inputs/IA_MoveHorizontal.IA_MoveHorizontal"))
  (Variables|Default|SetLocation_Desired (+ (Variables|Default|GetLocation_Desired) (* (Transformation|GetActorForwardVector) (* ActionValue (/ (Variables|/Script/Engine.SpringArmComponent|GetTargetArmLength (Variables|Default|GetSpringArm)) 5e+01))))))

(event Input|EnhancedActionEvents|EnhancedInputActionIA_MoveVertical
  (params (ActionValue :type Float%20%28double-precision%29) (ElapsedSeconds :type Float%20%28double-precision%29) (TriggeredSeconds :type Float%20%28double-precision%29) (InputAction :type Input%20Action%20Object%20Reference :default "/Game/Blueprints/Core/Player/Inputs/IA_MoveVertical.IA_MoveVertical"))
  (Variables|Default|SetLocation_Desired (+ (Variables|Default|GetLocation_Desired) (* (Transformation|GetActorRightVector) (* (/ (Variables|/Script/Engine.SpringArmComponent|GetTargetArmLength (Variables|Default|GetSpringArm)) 5e+01) ActionValue)))))

(event Input|EnhancedActionEvents|EnhancedInputActionIA_Rotate
  (params (ActionValue :type Float%20%28double-precision%29) (ElapsedSeconds :type Float%20%28double-precision%29) (TriggeredSeconds :type Float%20%28double-precision%29) (InputAction :type Input%20Action%20Object%20Reference :default "/Game/Blueprints/Core/Player/Inputs/IA_Rotate.IA_Rotate"))
  (:Started
    (Variables|Default|SetRotation_Desired (Math|Rotator|CombineRotators (Variables|Default|GetRotation_Desired) (Math|Rotator|MakeRotator 0.0 0.0 (* ActionValue 45.0))))))

(event EventBeginPlay
  (bind _asplayer_controller (Utilities|Casting|CastToPlayerController (Pawn|GetController)))
  (Utilities|IsValid (PlayerController|LocalPlayerSubsystems|GetEnhancedInputLocalPlayerSubsystem _asplayer_controller)
    (:Is%20Valid
      (Input|AddMappingContext (PlayerController|LocalPlayerSubsystems|GetEnhancedInputLocalPlayerSubsystem _asplayer_controller) "/Game/Blueprints/Core/Player/Inputs/IMC_PC.IMC_PC" 0 "(bIgnoreAllPressedKeysUntilRelease=True,bForceImmediately=False,bNotifyUserSettings=False)")
      (Variables|Default|SetLocation_Desired (Transformation|GetActorLocation))
      (Variables|Default|SetZoom_Desired (Variables|/Script/Engine.SpringArmComponent|GetTargetArmLength (Variables|Default|GetSpringArm)))
      (Variables|Default|SetRotation_Desired (Transformation|GetActorRotation)))))

(event EventTick
  (params (DeltaSeconds :type Float%20%28single-precision%29))
  (bind _springarm (Variables|Default|GetSpringArm))
  (Variables|/Script/Engine.SpringArmComponent|SetTargetArmLength _springarm (Math|Interpolation|FInterpTo (Variables|/Script/Engine.SpringArmComponent|GetTargetArmLength _springarm) (Variables|Default|GetZoom_Desired) DeltaSeconds 1e+01))
  (Transformation|SetActorLocation (Math|Interpolation|VInterpTo (Transformation|GetActorLocation) (Variables|Default|GetLocation_Desired) DeltaSeconds 1e+01) false false)
  (Transformation|SetActorRotation (Math|Interpolation|RInterpTo (Transformation|GetActorRotation) (Variables|Default|GetRotation_Desired) DeltaSeconds 1e+01)))

(fn ConstructionScript)